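; Maze door that opens with a specific skull key held by the player.
; Overlapping its trigger shows a HUD prompt, enabling Interact input only when the player has the matching key.
; Interacting lowers the key count, updates the HUD, attaches a spawned key mesh to the keyhole and plays a sound while a timeline moves key and door.
; The construction script applies the skull material to the door as a dynamic instance.
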(event OnComponentBeginOverlap(TriggerVolume)
  (params (OverlappedComponent :type Primitive%20Component%20Object%20Reference) (OtherActor :type Actor%20Object%20Reference) (OtherComp :type Primitive%20Component%20Object%20Reference) (OtherBodyIndex :type Integer) (bFromSweep :type Boolean) (SweepResult :type Hit%20Result%20Structure%20%28by%20ref%29))
  (if (== OtherActor (Game|GetPlayerCharacter 0))
    (if (not (Variables|Default|GetIsOpen))
      (if (not (Variables|Default|GetIsOpening))
        (bind _asplayer_character (Utilities|Casting|CastToPlayerCharacter (Game|GetPlayerCharacter 0)))
        (if (> (Variables|/Game/Player/PlayerCharacter.PlayerCharacter_C|GetNumberOfKeys _asplayer_character) 0)
          (bind _asplayer_character_2 (Utilities|Casting|CastToPlayerCharacter (Game|GetPlayerCharacter 0)))
          (if (Utilities|Array|ContainsItem (Variables|/Game/Player/PlayerCharacter.PlayerCharacter_C|GetOwnedKeys _asplayer_character_2) (Variables|Default|GetKeyRequired))
            (Input|EnableInput (Game|GetPlayerController 0))
            (bind _asmaze_game_mode (Utilities|Casting|CastToMazeGameMode (Game|GetGameMode)))
            (Variables|/Game/UI/HeadsUpDisplay.HeadsUpDisplay_C|SetMessage (Variables|/Game/GameSettings/MazeGameMode.MazeGameMode_C|GetHeadsUpDisplay _asmaze_game_mode) "Press 'E' to Open Door")
            (Default|UpdateMessage (Variables|/Game/GameSettings/MazeGameMode.MazeGameMode_C|GetHeadsUpDisplay _asmaze_game_mode))
            (else
              (bind _asmaze_game_mode_2 (Utilities|Casting|CastToMazeGameMode (Game|GetGameMode)))
              (Variables|/Game/UI/HeadsUpDisplay.HeadsUpDisplay_C|SetMessage (Variables|/Game/GameSettings/MazeGameMode.MazeGameMode_C|GetHeadsUpDisplay _asmaze_game_mode_2) "You don't have the right key for this door")
              (Default|UpdateMessage (Variables|/Game/GameSettings/MazeGameMode.MazeGameMode_C|GetHeadsUpDisplay _asmaze_game_mode_2))))
          (else
            (bind _asmaze_game_mode_3 (Utilities|Casting|CastToMazeGameMode (Game|GetGameMode)))
            (Variables|/Game/UI/HeadsUpDisplay.HeadsUpDisplay_C|SetMessage (Variables|/Game/GameSettings/MazeGameMode.MazeGameMode_C|GetHeadsUpDisplay _asmaze_game_mode_3) "Door Requires a Skull Key")
            (Default|UpdateMessage (Variables|/Game/GameSettings/MazeGameMode.MazeGameMode_C|GetHeadsUpDisplay _asmaze_game_mode_3))))))))

(event OnComponentEndOverlap(TriggerVolume)
  (params (OverlappedComponent :type Primitive%20Component%20Object%20Reference) (OtherActor :type Actor%20Object%20Reference) (OtherComp :type Primitive%20Component%20Object%20Reference) (OtherBodyIndex :type Integer))
  (if (not (== OverlappedComponent (Game|GetPlayerCharacter 0)))
    (Input|DisableInput (Game|GetPlayerController 0))
    (bind _asmaze_game_mode (Utilities|Casting|CastToMazeGameMode (Game|GetGameMode)))
    (Variables|/Game/UI/HeadsUpDisplay.HeadsUpDisplay_C|SetMessage (Variables|/Game/GameSettings/MazeGameMode.MazeGameMode_C|GetHeadsUpDisplay _asmaze_game_mode) "")
    (Default|UpdateMessage (Variables|/Game/GameSettings/MazeGameMode.MazeGameMode_C|GetHeadsUpDisplay _asmaze_game_mode))))

(event Input|ActionEvents|InputActionInteract
  (params (Key :type Key%20Structure :default "None"))
  (bind _keyrequired (Variables|Default|GetKeyRequired))
  (:Pressed
    (bind _asplayer_character (Utilities|Casting|CastToPlayerCharacter (Game|GetPlayerCharacter 0)))
    (if (> (Variables|/Game/Player/PlayerCharacter.PlayerCharacter_C|GetNumberOfKeys _asplayer_character) 0)
      (bind _asplayer_character_2 (Utilities|Casting|CastToPlayerCharacter (Game|GetPlayerCharacter 0)))
      (if (Utilities|Array|ContainsItem (Variables|/Game/Player/PlayerCharacter.PlayerCharacter_C|GetOwnedKeys _asplayer_character_2) _keyrequired)
        (Development|PrintString _keyrequired)
        (Development|PrintString "Found")
        (Math|Integer|DecrementInt (Variables|/Game/Player/PlayerCharacter.PlayerCharacter_C|GetNumberOfKeys _asplayer_character)
          (:%20%20
            (bind _asmaze_game_mode (Utilities|Casting|CastToMazeGameMode (Game|GetGameMode)))
            (Variables|/Game/UI/HeadsUpDisplay.HeadsUpDisplay_C|SetMessage (Variables|/Game/GameSettings/MazeGameMode.MazeGameMode_C|GetHeadsUpDisplay _asmaze_game_mode) "")
            (Default|UpdateMessage (Variables|/Game/GameSettings/MazeGameMode.MazeGameMode_C|GetHeadsUpDisplay _asmaze_game_mode))
            (Variables|Default|SetIsOpening true)
            (bind _asmaze_game_mode_2 (Utilities|Casting|CastToMazeGameMode (Game|GetGameMode)))
            (Default|UpdateSkulls (Variables|/Game/GameSettings/MazeGameMode.MazeGameMode_C|GetHeadsUpDisplay _asmaze_game_mode_2))
            (bind _returnvalue (AddComponent|AddStaticMeshComponent false))
            (bind _output_get (Variables|Default|SetKeyMesh _returnvalue))
            (Rendering|Material|SetMaterial _output_get 0 (Variables|Default|GetSkullMaterial))
            (Transformation|AttachComponentToComponent _output_get (Variables|Default|GetKeyhole) "None" "SnapToTarget" "SnapToTarget" "SnapToTarget" true)
            (Audio|PlaySoundatLocation "/Game/Audio/DoorOpening_SFX.DoorOpening_SFX" (Transformation|GetActorLocation) "0, 0, 0" 1.0 1.0 0.0 0 0 0 0)
            (bind (_direction _doorposition _keyposition) (Timeline|DoorOpening PlayFromStart)
              (:Update
                (Transformation|SetRelativeLocation (Variables|Default|GetKeyMesh) (Math|Vector|MakeVector 0.0 _keyposition 0.0) false false)
                (Transformation|SetRelativeLocation (Variables|Default|GetDoorMesh) (Math|Vector|MakeVector 0.0 0.0 _doorposition) false false))
              (:Finished
                (Variables|Default|SetIsOpen true)))))))))

(fn ConstructionScript
  (Rendering|Material|CreateDynamicMaterialInstance (Variables|Default|GetDoorMesh) 1 (Variables|Default|GetSkullMaterial) "None" :!class /Script/Engine.PrimitiveComponent))