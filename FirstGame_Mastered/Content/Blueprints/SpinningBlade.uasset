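; Spinning blade hazard that travels along a path and damages the player on contact.
; The gear mesh spins about its pitch axis each tick while the Movement timeline slides it toward EndPoint, with play rate scaled by distance to respect MovementSpeed.
; Box overlap launches a living player away from the actor's origin, deals damage, flags RecentlyDamaged and plays a hit sound.
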(event OnComponentBeginOverlap(Box)
  (params (OverlappedComponent :type Primitive%20Component%20Object%20Reference) (OtherActor :type Actor%20Object%20Reference) (OtherComp :type Primitive%20Component%20Object%20Reference) (OtherBodyIndex :type Integer) (bFromSweep :type Boolean) (SweepResult :type Hit%20Result%20Structure%20%28by%20ref%29))
  (bind _returnvalue (Game|GetPlayerCharacter 0))
  (bind _returnvalue_2 (Game|GetPlayerCharacter 0))
  (if (== OtherActor _returnvalue)
    (bind _asplayer_character (Utilities|Casting|CastToPlayerCharacter _returnvalue))
    (if (> (Variables|/Game/Player/PlayerCharacter.PlayerCharacter_C|GetHealth _asplayer_character) 0)
      (Character|LaunchCharacter _asplayer_character (* (Math|Vector|GetUnitDirection(Vector) (Transformation|GetActorLocation) (Transformation|GetActorLocation _returnvalue)) (Variables|Default|GetKnockbackStrength)) true true)
      (Game|Damage|ApplyDamage _asplayer_character 1.0 0 0)
      (bind _asplayer_character_2 (Utilities|Casting|CastToPlayerCharacter _returnvalue_2))
      (Variables|/Game/Player/PlayerCharacter.PlayerCharacter_C|SetRecentlyDamaged _asplayer_character_2 true)
      (Audio|PlaySoundatLocation "/Game/Audio/Hit_SFX.Hit_SFX" (Transformation|GetActorLocation _returnvalue_2) "0, 0, 0" 1.0 1.0 0.0 0 0 0 0))))

(event EventTick
  (params (DeltaSeconds :type Float%20%28single-precision%29))
  (Transformation|AddLocalRotation (Variables|Default|GetGearMesh) (Math|Rotator|MakeRotator 0.0 (* DeltaSeconds (Variables|Default|GetSpin%20Value)) 0.0) false false))

(event EventBeginPlay
  (Components|Timeline|SetPlayRate (Variables|Default|GetMovement) (/ (/ (Variables|Default|GetMovementSpeed) 1e+02) (/ (Math|Vector|VectorLength (Variables|Default|GetEndPoint)) 1e+02)))
  (bind _position (Timeline|Movement Play)
    (:Update
      (Transformation|SetRelativeLocation (Variables|Default|GetGearMesh) (* _position (Variables|Default|GetEndPoint)) false false))))

(fn ConstructionScript)