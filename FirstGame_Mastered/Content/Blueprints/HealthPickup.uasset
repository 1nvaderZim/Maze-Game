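; Health pickup actor for a maze game that restores one point of player health, shown as a star mesh.
; When the player character overlaps its collision, it adds health only if the current value is not above a small cap, then refreshes the HUD through MazeGameMode.
; It destroys only the star mesh, whose validity check prevents repeat pickups, so the actor itself remains.
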(event OnComponentBeginOverlap(collision)
  (params (OverlappedComponent :type Primitive%20Component%20Object%20Reference) (OtherActor :type Actor%20Object%20Reference) (OtherComp :type Primitive%20Component%20Object%20Reference) (OtherBodyIndex :type Integer) (bFromSweep :type Boolean) (SweepResult :type Hit%20Result%20Structure%20%28by%20ref%29))
  (if (== OtherActor (Game|GetPlayerCharacter 0))
    (Utilities|IsValid (Variables|Default|GetStarMesh)
      (:Is%20Valid
        (bind _asplayer_character (Utilities|Casting|CastToPlayerCharacter (Game|GetPlayerCharacter 0)))
        (if (not (> (Variables|/Game/Player/PlayerCharacter.PlayerCharacter_C|GetHealth _asplayer_character) 2))
          (Components|DestroyComponent (Variables|Default|GetStarMesh))
          (Math|Integer|IncrementInt (Variables|/Game/Player/PlayerCharacter.PlayerCharacter_C|GetHealth _asplayer_character)
            (:%20%20
              (bind _asplayer_character_2 (Utilities|Casting|CastToPlayerCharacter (Game|GetPlayerCharacter 0)))
              (Variables|/Game/Player/PlayerCharacter.PlayerCharacter_C|SetHealth _asplayer_character_2 (Variables|/Game/Player/PlayerCharacter.PlayerCharacter_C|GetHealth _asplayer_character_2))
              (bind _asmaze_game_mode (Utilities|Casting|CastToMazeGameMode (Game|GetGameMode)))
              (Default|UpdateHealth (Variables|/Game/GameSettings/MazeGameMode.MazeGameMode_C|GetHeadsUpDisplay _asmaze_game_mode)))))))))

(fn ConstructionScript)