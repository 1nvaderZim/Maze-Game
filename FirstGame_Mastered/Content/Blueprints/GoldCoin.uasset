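; GoldCoin is a collectible coin that adds its CoinValue to the player's score when picked up.
; On BeginPlay a timeline animates the mesh, moving it vertically and spinning it in yaw each update.
; When the player character overlaps the sphere, it adds to Score, destroys only the mesh component, stops the timeline and refreshes the MazeGameMode HUD score.
; The mesh validity check prevents repeat scoring, as the actor itself remains.
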(event OnComponentBeginOverlap(Sphere)
  (params (OverlappedComponent :type Primitive%20Component%20Object%20Reference) (OtherActor :type Actor%20Object%20Reference) (OtherComp :type Primitive%20Component%20Object%20Reference) (OtherBodyIndex :type Integer) (bFromSweep :type Boolean) (SweepResult :type Hit%20Result%20Structure%20%28by%20ref%29))
  (bind _returnvalue (Game|GetPlayerCharacter 0))
  (if (== OtherActor _returnvalue)
    (Utilities|IsValid (Variables|Default|GetCoinMesh)
      (:Is%20Valid
        (bind _asplayer_character (Utilities|Casting|CastToPlayerCharacter _returnvalue))
        (Variables|/Game/Player/PlayerCharacter.PlayerCharacter_C|SetScore _asplayer_character (+ (Variables|/Game/Player/PlayerCharacter.PlayerCharacter_C|GetScore _asplayer_character) (Variables|Default|GetCoinValue)))
        (Components|DestroyComponent (Variables|Default|GetCoinMesh))
        (Audio|Components|Audio|Stop (Variables|Default|GetCoinTimeline))
        (bind _asmaze_game_mode (Utilities|Casting|CastToMazeGameMode (Game|GetGameMode)))
        (Default|UpdateScore (Variables|/Game/GameSettings/MazeGameMode.MazeGameMode_C|GetHeadsUpDisplay _asmaze_game_mode))))))

(event Custom|AnimateCoin
  (Utilities|IsValid (Variables|Default|GetCoinMesh)
    (:Is%20Valid
      (bind _position (Timeline|CoinTimeline Play)
        (:Update
          (Transformation|SetRelativeLocation (Variables|Default|GetCoinMesh) (Math|Vector|MakeVector 0.0 0.0 (.z _position)) false false)
          (Transformation|AddLocalRotation (Variables|Default|GetCoinMesh) "1.000000,0.000000,0.000000" false false))))))

(event EventBeginPlay
  (CallFunction|AnimateCoin))

(event Collision|EventActorBeginOverlap
  (params (OtherActor :type Actor%20Object%20Reference)))

(event EventTick
  (params (DeltaSeconds :type Float%20%28single-precision%29)))

(fn ConstructionScript)